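; PC_game is a player controller that sets up input, the HUD and an inventory menu toggle.
; On BeginPlay, if the Enhanced Input subsystem is valid, it adds IMC_Default and puts UI_HUD on screen.
; The IA_inventaire action creates or removes the UI_menu widget, showing or hiding the mouse cursor with it.
; Opening the menu also prints a debug "Hello".
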(event `self.ReceiveBeginPlay`
  (bind _returnvalue (subsystem `EnhancedInputLocalPlayerSubsystem`))
  (`/Engine/EditorBlueprintResources/StandardMacros.IsValid` _returnvalue
    (:`Is Valid`
      (`EnhancedInputSubsystemInterface.AddMappingContext` _returnvalue "/Game/111_JITON/Input/IMC_Default.IMC_Default" 0 (struct))
      (bind _returnvalue_2 (`|CreateWidget` "/Game/111_JITON/UI/UI_HUD.UI_HUD_C"))
      (bind _output_get (set `self.UI_hud` _returnvalue_2))
      (`UserWidget.AddToViewport` _output_get 0))))

(event `EnhancedInput|/Game/111_JITON/Input/Actions/IA_inventaire`
  (params (ActionValue :type Boolean) (ElapsedSeconds :type "Float (double-precision)") (TriggeredSeconds :type "Float (double-precision)") (InputAction :type "InputAction Object Reference" :default "/Game/111_JITON/Input/Actions/IA_inventaire.IA_inventaire"))
  (:`Triggered`
    (bind _ui_inventaire (`self.UI_inventaire`)
      (:`then`
        (`Widget.RemoveFromParent` _ui_inventaire)
        (set `self.UI_inventaire` null)
        (set `self.bShowMouseCursor` false))
      (:`else`
        (bind _returnvalue (`|CreateWidget` "/Game/111_JITON/UI/informations/UI_menu.UI_menu_C"))
        (bind _output_get (set `self.UI_inventaire` _returnvalue))
        (`UserWidget.AddToViewport` _output_get 0)
        (set `self.bShowMouseCursor` true)
        (`KismetSystemLibrary.PrintString` "Hello")))))

(fn `UserConstructionScript`)